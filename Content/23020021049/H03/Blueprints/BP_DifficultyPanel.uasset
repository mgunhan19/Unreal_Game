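; BP_DifficultyPanel is an actor meant to select one of four difficulty levels from number keys 1 to 4.
; It enables input for player controller 0 on BeginPlay, and each key press looks up an actor of its own class.
; The ApplyDifficulty calls for indices 0 to 3 are not connected to execution, so the keys currently apply no difficulty.
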(event Collision|EventActorBeginOverlap
  (params (OtherActor :type Actor%20Object%20Reference)))

(event EventTick
  (params (DeltaSeconds :type Float%20%28single-precision%29)))

(event EventBeginPlay
  (Input|EnableInput (Game|GetPlayerController 0)))

(event Input|KeyboardEvents|1
  (params (Key :type Key%20Structure :default "None"))
  (:Pressed
    (bind _returnvalue (Actor|GetActorOfClass "BP_DifficultyPanel_C"))))

(event Input|KeyboardEvents|2
  (params (Key :type Key%20Structure :default "None"))
  (:Pressed
    (bind _returnvalue (Actor|GetActorOfClass "BP_DifficultyPanel_C"))))

(event Input|KeyboardEvents|3
  (params (Key :type Key%20Structure :default "None"))
  (:Pressed
    (bind _returnvalue (Actor|GetActorOfClass "BP_DifficultyPanel_C"))))

(event Input|KeyboardEvents|4
  (params (Key :type Key%20Structure :default "None"))
  (:Pressed
    (bind _returnvalue (Actor|GetActorOfClass "BP_DifficultyPanel_C"))))

(fn ConstructionScript)