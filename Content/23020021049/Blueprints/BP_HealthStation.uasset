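; BP_HealthStation is a health station that starts a looping timer when a Character overlaps it.
; Each fast tick runs CanDoldur, adding to the station's own Can (health) variable without a clamp and printing it.
; End overlap clears TimerHandleCan and prints an exit message, but that handle's assignment is unconnected, so the started timer keeps running.
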(event Custom|Can%20Doldur
  (Variables|Default|SetCan (+ (Variables|Default|GetCan) 1e+02))
  (Development|PrintString (Utilities|String|Append "Can:" (Utilities|String|ToString(Float) (Variables|Default|GetCan))) true true "(R=0.000000,G=0.660000,B=1.000000,A=1.000000)" 2.0 "Can"))

(event Collision|EventActorEndOverlap
  (params (OtherActor :type Actor%20Object%20Reference))
  (Utilities|Casting|CastToCharacter OtherActor)
  (Utilities|Time|ClearandInvalidateTimerbyHandle (Variables|Default|GetTimerHandle_Can))
  (Development|PrintString "Can istasyonundan ciktin" true true "(R=0.000000,G=0.660000,B=1.000000,A=1.000000)" 2.0 "Can"))

(event Collision|EventActorBeginOverlap
  (params (OtherActor :type Actor%20Object%20Reference))
  (Utilities|Casting|CastToCharacter OtherActor)
  (bind _returnvalue (Utilities|Time|SetTimerbyEvent (delegate Custom|Can%20Doldur) 0.05 true)))

(fn ConstructionScript)