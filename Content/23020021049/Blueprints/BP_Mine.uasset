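; BP_Mine is a mine actor that launches an overlapping Character straight upward and then hides itself.
; A DoOnce limits it to a single trigger, and pressing R, through input enabled for player 0 at BeginPlay, unhides the mine and rearms it.
; Collision stays untouched while it is hidden, as the nodes for toggling trigger collision and printing a rearm message are not wired to run.
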(event EventBeginPlay
  (Input|EnableInput (Game|GetPlayerController 0)))

(event Collision|EventActorBeginOverlap
  (params (OtherActor :type Actor%20Object%20Reference))
  (bind _ascharacter (Utilities|Casting|CastToCharacter OtherActor))
  (Utilities|FlowControl|DoOnce false
    (:Completed
      (Character|LaunchCharacter _ascharacter "0.000000,0.000000,1500.000000" false true)
      (Rendering|SetActorHiddenInGame true))))

(event Input|KeyboardEvents|R
  (params (Key :type Key%20Structure :default "None"))
  (:Pressed
    (Rendering|SetActorHiddenInGame false)
    (Utilities|FlowControl|DoOnce false) ; enters at Reset
  ))

(fn ConstructionScript)