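; BP_DifficultyPanel is an actor that maps number keys 1 to 4 to a difficulty selection.
; It enables input from player controller 0 on BeginPlay, and each key press calls ApplyDifficulty.
; ApplyDifficulty switches on Level to print a Turkish label with an enemy count, without spawning enemies or storing the choice.
; All four keys currently pass Level 0, so only the easy message ever appears.
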(event EventBeginPlay
  (Input|EnableInput (Game|GetPlayerController 0)))

(event Collision|EventActorBeginOverlap
  (params (OtherActor :type Actor%20Object%20Reference)))

(event EventTick
  (params (DeltaSeconds :type Float%20%28single-precision%29)))

(event Input|KeyboardEvents|1
  (params (Key :type Key%20Structure :default "None"))
  (:Pressed
    (CallFunction|ApplyDifficulty)))

(event Input|KeyboardEvents|2
  (params (Key :type Key%20Structure :default "None"))
  (:Pressed
    (CallFunction|ApplyDifficulty)))

(event Input|KeyboardEvents|3
  (params (Key :type Key%20Structure :default "None"))
  (:Pressed
    (CallFunction|ApplyDifficulty)))

(event Input|KeyboardEvents|4
  (params (Key :type Key%20Structure :default "None"))
  (:Pressed
    (CallFunction|ApplyDifficulty)))

(fn ConstructionScript)

(fn ApplyDifficulty
  (params (Level :type Integer))
  (switch int Level
    (:0
      (Development|PrintString "Kolay: 5 dusman" true true "(R=0.000000,G=0.660000,B=1.000000,A=1.000000)" 2.0 "Zorluk"))
    (:1
      (Development|PrintString "Orta: 10 dusman" true true "(R=0.000000,G=0.660000,B=1.000000,A=1.000000)" 2.0 "Zorluk"))
    (:2
      (Development|PrintString "Zor: 15 düşman" true true "(R=0.000000,G=0.660000,B=1.000000,A=1.000000)" 2.0 "Zorluk"))
    (:3
      (Development|PrintString "Cok Zor: 25 dusman" true true "(R=0.000000,G=0.660000,B=1.000000,A=1.000000)" 2.0 "Zorluk"))))