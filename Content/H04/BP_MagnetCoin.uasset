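; BP_MagnetCoin is a spinning coin pickup that prints a message and destroys itself when a Character overlaps it.
; Tick rotates it around yaw and, within PullRadius, applies a Speed-scaled move intended as a magnet pull.
; As wired, distance and direction are both measured against the coin itself, so the pull produces no movement.
; The Get Player Character node is left unconnected.
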(event Collision|EventActorBeginOverlap
  (params (OtherActor :type Actor%20Object%20Reference))
  (Utilities|Casting|CastToCharacter OtherActor)
  (Development|PrintString "Coin Tplandi")
  (Actor|DestroyActor))

(event EventTick
  (params (DeltaSeconds :type Float%20%28single-precision%29))
  (bind _returnvalue (Transformation|GetActorLocation))
  (Transformation|AddActorLocalRotation (Math|Rotator|MakeRotator 0.0 0.0 (* 1.8e+02 DeltaSeconds)) false false)
  (if (< (Transformation|GetDistanceTo self) (Variables|Default|GetPullRadius))
    (Transformation|SetActorLocation (+ _returnvalue (* (Math|Vector|GetUnitDirection(Vector) _returnvalue (Transformation|GetActorLocation)) (* (Variables|Default|GetSpeed) DeltaSeconds))) false false)))

(fn ConstructionScript)