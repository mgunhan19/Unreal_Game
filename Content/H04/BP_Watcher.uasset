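; BP_Watcher is a stationary-logic sentry that detects when the player character enters its forward view cone.
; Each tick, CanSeePlayer combines a distance check against ViewDistance with a forward dot product against ConeDot, without any line-of-sight trace.
; The result swaps the Cylinder between alert and calm materials and prints a "seen" message in Turkish.
; A debug cone visualizes the view range from a raised origin every frame.
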(event EventBeginPlay)

(event Collision|EventActorBeginOverlap
  (params (OtherActor :type Actor%20Object%20Reference)))

(event EventTick
  (params (DeltaSeconds :type Float%20%28single-precision%29))
  (Class|KismetSystemLibrary|DrawDebugConeinDegrees (+ (Transformation|GetActorLocation) (Math|Vector|MakeVector 0.0 0.0 185.0)) (Transformation|GetActorForwardVector) (Variables|Default|GetViewDistance) 45.0 45.0 24 "(R=1.000000,G=0.795784,B=0.025081,A=1.000000)" 0.0 1.5 "World")
  (bind _seen (CallFunction|CanSeePlayer))
  (if _seen
    (Rendering|Material|SetMaterial (Variables|Default|GetCylinder) 0 "/Game/H04/MI_WatcherAlert.MI_WatcherAlert")
    (Development|PrintString "GÖRÜLDÜN")
    (else
      (Rendering|Material|SetMaterial (Variables|Default|GetCylinder) 0 "/Game/H04/MI_WatcherCalm.MI_WatcherCalm"))))

(fn ConstructionScript)

(fn CanSeePlayer
  (bind _returnvalue (Game|GetPlayerCharacter 0))
  (Variables|Default|SetDotValue 0.0)
  (return (and (< (Transformation|GetDistanceTo _returnvalue) (Variables|Default|GetViewDistance)) (> (Math|Vector|DotProduct (Transformation|GetActorForwardVector) (Math|Vector|GetUnitDirection(Vector) (Transformation|GetActorLocation) (Transformation|GetActorLocation _returnvalue))) (Variables|Default|GetConeDot)))))